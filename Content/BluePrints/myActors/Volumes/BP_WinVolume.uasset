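; BP_WinVolume is a level-exit volume that reacts when the player overlaps it.
; It quits the game if any Bp_Crystal actors remain in the world, and otherwise calls CompleteLevel.
; CompleteLevel finds the current level in the LevelNames array and opens the next one by name, doing nothing on the final level.
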(event `self.ReceiveActorBeginOverlap`
  (params (OtherActor :type "Actor Object Reference"))
  (`/Game/BluePrints/Libaries/CC_MacroLibrary.isPlayer` OtherActor
    (:`IsPlayer`
      (if (`self.Any Crystals Remaining`)
        ;[1 1 1] Quits the game once all the levels have been completed
        (`KismetSystemLibrary.QuitGame` null "Quit")
        (else
          ;[1 1 1] Hanlde loading new levels for the game
          (`self.Complete Level`))))))

(fn `Any Crystals Remaining`
  (returns (NewParam :type Boolean))
  (bind _outactors (`GameplayStatics.GetAllActorsOfClass` "/Game/BluePrints/myActors/Collectables/Bp_Crystal.Bp_Crystal_C"))
  (return (> (`KismetArrayLibrary.Array_Length` _outactors) 0)))

(fn `Complete Level`
  (if (not (`self.is final level`))
    (`self.Load Next Level`)))

(fn `Get Current Level Index`
  (returns (`Return Value` :type Integer))
  ;[1 1 1] Will get our current level name and try to find the current level within the array and will return the current index of it
  (bind _returnvalue (`GameplayStatics.GetCurrentLevelName` true))
  (return (`KismetArrayLibrary.Array_Find` (`self.Level Names`) (`KismetStringLibrary.Conv_StringToName` _returnvalue))))

(fn `Get Next Level Name`
  (returns (`Return Value` :type Name))
  (return (`|GetArrayItem` (`self.Level Names`) (+ (`self.Get Current Level Index`) 1))))

(fn `is final level`
  (returns (`Return Value` :type Boolean))
  (return (== (`KismetArrayLibrary.Array_LastIndex` (`self.Level Names`)) (`self.Get Current Level Index`))))

(fn `Load Next Level`
  (`GameplayStatics.OpenLevel` (`self.Get Next Level Name`)))

(fn `UserConstructionScript`)